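; BP_LevelData is a level settings actor that can lock the player's view to a static camera.
; On BeginPlay it finds all BP_LevelData actors and, unless duplicates exist, reads the CameraLock flag.
; When locked, it finds the level's BP_StaticCam and makes it the first player controller's view target.
; Duplicate level data or static camera actors only print a warning and leave the view unchanged.
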(event `self.ReceiveBeginPlay`
  ;[1 1 1] Handle Level Data, Why did i ever write this in the character controller and not the Level Data actor?????? Am i actually disabled????
  (bind _outactors (`GameplayStatics.GetAllActorsOfClass` "BP_LevelData_C"))
  (if (>= (`KismetArrayLibrary.Array_Length` _outactors) 2)
    (`KismetSystemLibrary.PrintString` "More then 1 Level Data present in current scene! Defaulting to None.")
    (elif (`/Game/Core/Blueprints/Level/BP_LevelData.CameraLock` (`|GetArrayItem` _outactors))
      (bind _outactors_2 (`GameplayStatics.GetAllActorsOfClass` "/Game/Core/Blueprints/Level/BP_StaticCam.BP_StaticCam_C"))
      (if (>= (`KismetArrayLibrary.Array_Length` _outactors_2) 2)
        (`KismetSystemLibrary.PrintString` "More then 1 Static Camera  present in current scene! Defaulting to None.")
        (else
          (`PlayerController.SetViewTargetWithBlend` (`GameplayStatics.GetPlayerController` 0) (`|GetArrayItem` _outactors_2) 0.0 "VTBlend_Linear" 0.0 false))))))

(fn `UserConstructionScript`)