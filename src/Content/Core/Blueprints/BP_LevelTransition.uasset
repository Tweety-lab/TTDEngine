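; BP_LevelTransition is a trigger actor that moves the game to another level when the first player's pawn overlaps it.
; On overlap it fades the camera and audio out, holds the fade, waits for it to finish, then opens TargetLevel by name.
; The construction script clears either ExitID or the TargetLevel and TargetExit pair depending on Direction, and the overlap logic reads neither Direction nor the exit fields.
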(event `self.ReceiveActorBeginOverlap`
  (params (OtherActor :type "Actor Object Reference"))
  ;[1 1 1] Incredibly stupid fading system, Valve please fix
  (if (== OtherActor (`GameplayStatics.GetPlayerPawn` 0))
    (`PlayerCameraManager.StartCameraFade` :`self` (`GameplayStatics.GetPlayerCameraManager` 0) :`ToAlpha` 1.0 :`Duration` 0.3 :`bShouldFadeAudio` true :`bHoldWhenFinished` true)
    (`KismetSystemLibrary.Delay` 0.3)
    (`GameplayStatics.OpenLevel` (`KismetStringLibrary.Conv_StringToName` (`self.Target Level`)))))

(fn `UserConstructionScript`
  (if (`|EnumInequality` (`self.Direction`) "NewEnumerator1")
    (if (not (`|EnumInequality` (`self.Direction`) "NewEnumerator0"))
      (set `self.Exit ID` ""))
    (else
      (set `self.Target Level` "")
      (set `self.Target Exit` ""))))